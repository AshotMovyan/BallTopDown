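; Actor component that spawns a group of enemies around its owner and signals when all of them are dead.
; On BeginPlay it spawns a BP_Enemy at each Points offset from the owner's location, stores it and binds to its OnDestroyed event.
; A destroyed counter triggers the EnemiesAreDead dispatcher once it reaches the spawned count.
; The EnemyClass variable is unused, as the spawned class is hardcoded.
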(event `self.ReceiveBeginPlay`
  (for _array_element (`self.Points`)
    (bind _returnvalue (`|SpawnActorFromClass` "/Game/BluePrints/Enemy/BP_Enemy.BP_Enemy_C" (`KismetMathLibrary.MakeTransform` (+ (`Actor.K2_GetActorLocation` (`self.GetOwner`)) _array_element)) "Undefined" "OverrideRootScale" null null))
    (`KismetArrayLibrary.Array_Add` (`self.Enemies`) _returnvalue)
    (add `Actor.OnDestroyed` _returnvalue (delegate `OnEnemyDestroyed`))))

(event `OnEnemyDestroyed`
  (params (DestroyedActor :type "Actor Object Reference"))
  (bind _result (`/Engine/EditorBlueprintResources/StandardMacros.IncrementInt` (`self.DestroyedEnemies`))
    (:`  `
      (if (>= _result (`KismetArrayLibrary.Array_Length` (`self.Enemies`)))
        (`self.EnemiesAreDead`)))))